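; EnemyAI is an AI controller Blueprint that starts the enemy's behavior tree.
; On BeginPlay it loads the EnemyBB blackboard, stores player controller 0 (not the pawn) in PlayerKey, then runs EnemyBehaviour.
; An unconnected leftover patrol loop, which moves to random TargetPoints with a three-second delay, never executes.
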(event EventBeginPlay
  (bind _blackboardcomponent (Class|AIController|UseBlackboard "/Game/Blueprints/AI/EnemyBB.EnemyBB"))
  (AI|Components|Blackboard|SetValueasObject _blackboardcomponent (Variables|Default|GetPlayerKey) (Game|GetPlayerController 0))
  (AI|RunBehaviorTree "/Game/Blueprints/AI/EnemyBehaviour.EnemyBehaviour"))

(fn ConstructionScript)