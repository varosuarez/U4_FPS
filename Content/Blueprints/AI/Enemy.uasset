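; Zombie enemy character that attacks the player in range, takes damage from first-person projectiles and maintains the player's enemy count.
; Tick updates the widget health bar, sets the anim Blueprint's attack flag by distance, and uses a Delay to pace damage to the player.
; Projectile hits play explosion effects and subtract the player's Damage from Health.
; At minimum health it triggers death animation, then decrements player and spawner counters before destroying itself.
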(event EventBeginPlay
  ;[1 1 1] Add enemy on start
  (bind _asfirst_person_character (Utilities|Casting|CastToFirstPersonCharacter (Game|GetPlayerCharacter 0)))
  (Variables|Default|SetPlayerReference _asfirst_person_character)
  (Math|Integer|IncrementInt (Variables|/Game/Blueprints/FirstPersonCharacter.FirstPersonCharacter_C|GetEnemies _asfirst_person_character)))

(event Collision|EventActorBeginOverlap
  (params (OtherActor :type Actor%20Object%20Reference)))

(event EventTick
  (params (DeltaSeconds :type Float%20%28single-precision%29))
  (bind _generatedby (Variables|Default|GetGeneratedBy))
  ;[1 1 1] Check if health is = 0
  (if (> (Variables|Default|GetHealth) (Variables|Default|GetMinHealth))
    ;[1 1 1] HUD Health Bar
    (bind _asenemy_health_bar (Utilities|Casting|CastToEnemyHealthBar (UserInterface|GetUserWidgetObject (Variables|Default|GetHealthBar))))
    (Progress|SetPercent (Variables|/Game/Blueprints/Widgets/EnemyHealthBar.EnemyHealthBar_C|GetHealthBar _asenemy_health_bar) (Variables|Default|GetHealth))
    ;[1 1 1] Attack Logic
    (bind _asfirst_person_character (Utilities|Casting|CastToFirstPersonCharacter (Game|GetPlayerCharacter 0)))
    (bind _aszombie_anim_bp (Utilities|Casting|CastToZombieAnimBP (Components|SkeletalMesh|GetAnimInstance (Variables|Character|GetMesh))))
    (bind _output_get (Variables|/Game/Blueprints/AI/ZombieAnimBP.ZombieAnimBP_C|SetisAttacking _aszombie_anim_bp (<= (Transformation|GetDistanceTo _asfirst_person_character) (Variables|Default|GetAttackRange))))
    (Utilities|FlowControl|Delay (Variables|Default|GetAttackSpeed))
    (if _output_get
      (if (>= (Variables|/Game/Blueprints/FirstPersonCharacter.FirstPersonCharacter_C|GetHealth _asfirst_person_character) 0.0)
        (Variables|/Game/Blueprints/FirstPersonCharacter.FirstPersonCharacter_C|SetHealth _asfirst_person_character (- (Variables|/Game/Blueprints/FirstPersonCharacter.FirstPersonCharacter_C|GetHealth _asfirst_person_character) (Variables|Default|GetDamage)))))
    (else
      ;[1 1 1] Death Animation
      (bind _aszombie_anim_bp_2 (Utilities|Casting|CastToZombieAnimBP (Components|SkeletalMesh|GetAnimInstance (Variables|Character|GetMesh))))
      (Variables|/Game/Blueprints/AI/ZombieAnimBP.ZombieAnimBP_C|SetisDead _aszombie_anim_bp_2 true)
      (Pawn|Components|CharacterMovement|DisableMovement (Variables|Character|GetCharacterMovement))
      ;[1 1 1] Hide Health Bar
      (Rendering|SetVisibility (Variables|Default|GetHealthBar) false false)
      ;[1 1 1] Destroy Enemy
      (Utilities|FlowControl|Delay 2.0)
      (Math|Integer|DecrementInt (Variables|/Game/Blueprints/FirstPersonCharacter.FirstPersonCharacter_C|GetEnemies (Variables|Default|GetPlayerReference))
        (:%20%20
          ;[1 1 1] Decrement the generated mob counter if spawn exists
          (Utilities|IsValid _generatedby
            (:Is%20Valid
              (Math|Integer|DecrementInt (Variables|/Game/Blueprints/MobGenerator.MobGenerator_C|GetGeneratedMobs _generatedby)
                (:%20%20
                  _)))
            (:Is%20Not%20Valid
              _))
          (Actor|DestroyActor))))))

(event Collision|EventHit
  (params (MyComp :type Primitive%20Component%20Object%20Reference) (Other :type Actor%20Object%20Reference) (OtherComp :type Primitive%20Component%20Object%20Reference) (bSelfMoved :type Boolean) (HitLocation :type Vector :default "0, 0, 0") (HitNormal :type Vector :default "0, 0, 0") (NormalImpulse :type Vector :default "0, 0, 0") (Hit :type Hit%20Result%20Structure%20%28by%20ref%29))
  (bind _returnvalue (Transformation|GetActorLocation))
  ;[1 1 1] OnHit Reduce Health
  (Utilities|Casting|CastToFirstPersonProjectile Other)
  (Audio|PlaySoundatLocation "/Game/StarterContent/Audio/Explosion01.Explosion01" _returnvalue "0, 0, 0" 1.0 1.0 0.0 0 0 0)
  (Effects|SpawnEmitteratLocation "/Game/StarterContent/Particles/P_Explosion.P_Explosion" _returnvalue)
  (bind _asfirst_person_character (Utilities|Casting|CastToFirstPersonCharacter (Game|GetPlayerCharacter 0)))
  (Variables|Default|SetHealth (Math|Float|Max(Float) (- (Variables|Default|GetHealth) (Variables|/Game/Blueprints/FirstPersonCharacter.FirstPersonCharacter_C|GetDamage _asfirst_person_character)) (Variables|Default|GetMinHealth))))

(fn ConstructionScript
  (|CallParentFunction))