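; Health pickup actor that restores health to the player's FirstPersonCharacter on contact.
; It spins continuously on all three axes every tick, scaled by delta time.
; On overlap with that character, it adds HealthAmount clamped to MaxHealth, plays a sound and explosion particle at its location, then destroys itself.
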(event EventBeginPlay)

(event Collision|EventActorBeginOverlap
  (params (OtherActor :type Actor%20Object%20Reference))
  (bind _returnvalue (Transformation|GetActorLocation))
  (bind _asfirst_person_character (Utilities|Casting|CastToFirstPersonCharacter OtherActor))
  (Variables|/Game/Blueprints/FirstPersonCharacter.FirstPersonCharacter_C|SetHealth _asfirst_person_character (Math|Float|Min(Float) (+ (Variables|/Game/Blueprints/FirstPersonCharacter.FirstPersonCharacter_C|GetHealth _asfirst_person_character) (Variables|Default|GetHealthAmount)) (Variables|/Game/Blueprints/FirstPersonCharacter.FirstPersonCharacter_C|GetMaxHealth _asfirst_person_character)))
  (Audio|PlaySoundatLocation "/Game/StarterContent/Audio/Collapse01.Collapse01" _returnvalue "0, 0, 0" 1.0 1.0 0.0 0 0 0)
  (Effects|SpawnEmitteratLocation "/Game/StarterContent/Particles/P_Explosion.P_Explosion" _returnvalue)
  (Actor|DestroyActor))

(event EventTick
  (params (DeltaSeconds :type Float%20%28single-precision%29))
  ;[1 1 1] Continuous rotate
  (Transformation|AddActorLocalRotation (* (Math|Rotator|MakeRotator 1.5e+02 72.0 1.5e+02) DeltaSeconds) false false))

(fn ConstructionScript)