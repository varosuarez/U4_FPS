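; Target actor that patrols along the X axis and is destroyed after taking enough projectile hits.
; Tick moves it along a normalized direction scaled by speed and delta time, while a Delay into a FlipFlop reverses direction about every three seconds.
; Each FirstPersonProjectile hit plays explosion effects and decrements health, swapping the material while health remains.
; At zero health it notifies the player's FirstPersonCharacter and destroys itself.
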(event Collision|EventActorBeginOverlap
  (params (OtherActor :type Actor%20Object%20Reference)))

(event EventTick
  (params (DeltaSeconds :type Float%20%28single-precision%29))
  (Transformation|SetActorLocation (+ (* (Math|Vector|Normalize (Variables|Test|GetDirection)) (* (Utilities|Time|GetWorldDeltaSeconds) (Variables|Test|GetSpeed))) (Transformation|GetActorLocation)) false false)
  (Utilities|FlowControl|Delay 3.0)
  (Utilities|FlowControl|FlipFlop
    (:A
      (Variables|Test|SetDirection "-1.000000, 0, 0"))
    (:B
      (Variables|Test|SetDirection "1.000000, 0, 0"))))

(event Collision|EventHit
  (params (MyComp :type Primitive%20Component%20Object%20Reference) (Other :type Actor%20Object%20Reference) (OtherComp :type Primitive%20Component%20Object%20Reference) (bSelfMoved :type Boolean) (HitLocation :type Vector :default "0, 0, 0") (HitNormal :type Vector :default "0, 0, 0") (NormalImpulse :type Vector :default "0, 0, 0") (Hit :type Hit%20Result%20Structure%20%28by%20ref%29))
  (bind _returnvalue (Transformation|GetActorLocation))
  (bind _health (Variables|Test|GetHealth))
  ;[1 1 1] OnHit cambio de material
  (Utilities|Casting|CastToFirstPersonProjectile Other)
  (Audio|PlaySoundatLocation "/Game/StarterContent/Audio/Explosion01.Explosion01" _returnvalue "0, 0, 0" 1.0 1.0 0.0 0 0 0)
  (Effects|SpawnEmitteratLocation "/Game/StarterContent/Particles/P_Explosion.P_Explosion" _returnvalue)
  (Math|Integer|DecrementInt _health
    (:%20%20
      (if (>= _health 1)
        (Rendering|Material|SetMaterial (Variables|Debug|GetStaticMeshComponent) 0 "/Game/Materials/Chicle.Chicle")
        (else
          (bind _asfirst_person_character (Utilities|Casting|CastToFirstPersonCharacter (Game|GetPlayerCharacter 0))
            (:then
              (Default|TargetDestroyTestEvent _asfirst_person_character))
            (:CastFailed
              _))
          (Actor|DestroyActor))))))

(fn ConstructionScript)