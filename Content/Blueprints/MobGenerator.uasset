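; MobGenerator is a destructible, constantly rotating spawner actor that produces Enemy mobs running EnemyBehaviour.
; Tick uses a Delay as a periodic gate, calling SpawnMob while GeneratedMobs is below MobsCap.
; SpawnMob places enemies at random offsets within SpawnRange at a fixed SpawnZ, setting GeneratedBy to itself.
; Projectile hits spawn explosions and reduce health, which regenerates through a retriggerable-delay loop until full, or destroy the actor at zero.
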(event Collision|EventHit
  (params (MyComp :type Primitive%20Component%20Object%20Reference) (Other :type Actor%20Object%20Reference) (OtherComp :type Primitive%20Component%20Object%20Reference) (bSelfMoved :type Boolean) (HitLocation :type Vector :default "0, 0, 0") (HitNormal :type Vector :default "0, 0, 0") (NormalImpulse :type Vector :default "0, 0, 0") (Hit :type Hit%20Result%20Structure%20%28by%20ref%29))
  (bind _currenthealth (Variables|Default|GetCurrentHealth))
  (bind _currenthealth_2 (Variables|Default|GetCurrentHealth))
  ;[1 1 1] If hit by projectile, decrease HP
  (Utilities|Casting|CastToFirstPersonProjectile Other)
  (Effects|SpawnEmitteratLocation "/Game/StarterContent/Particles/P_Explosion.P_Explosion" (Transformation|GetActorLocation))
  (Math|Integer|DecrementInt _currenthealth
    (:%20%20
      (if (>= _currenthealth 1)
        ;[1 1 1] Recover HP every 2 secs if not at maxHP
        (Utilities|FlowControl|RetriggerableDelay 2.0 :!label _label)
        (Math|Integer|IncrementInt _currenthealth_2
          (:%20%20
            (if (not (>= _currenthealth_2 (Variables|Default|GetMaxHealth)))
              (goto _label))))
        (else
          ;[1 1 1] Destruction effect
          (Actor|DestroyActor))))))

(event EventTick
  (params (DeltaSeconds :type Float%20%28single-precision%29))
  ;[1 1 1] Continuous rotate
  (Transformation|AddActorLocalRotation (* (Math|Rotator|MakeRotator 1.5e+02 72.0 1.5e+02) DeltaSeconds) false false)
  ;[1 1 1] Spawn mob every 3 secs if the cap isn't reached
  (Utilities|FlowControl|Delay 3.0)
  (if (< (Variables|Default|GetGeneratedMobs) (Variables|Default|GetMobsCap))
    (Math|Integer|IncrementInt (Variables|Default|GetGeneratedMobs)
      (:%20%20
        (CallFunction|SpawnMob)))))

(fn ConstructionScript)

(fn SpawnMob
  (bind _returnvalue (Transformation|GetActorLocation))
  (bind _returnvalue_2 (Class|KismetMathLibrary|VectorForward))
  (bind _returnvalue_3 (Math|Random|RandomFloatinRange 0.0 3.6e+02))
  (bind _spawnrange (Variables|Default|GetSpawnRange))
  (bind _returnvalue_4 (Math|Vector|RotateVector _returnvalue_2 (Math|Rotator|MakeRotator 0.0 0.0 _returnvalue_3)))
  (bind _returnvalue_5 (* _returnvalue_4 _spawnrange))
  (bind _returnvalue_6 (+ _returnvalue _returnvalue_5))
  (bind _returnvalue_7 (AI|SpawnAIFromClass "/Game/Blueprints/AI/Enemy.Enemy_C" "/Game/Blueprints/AI/EnemyBehaviour.EnemyBehaviour" (Math|Vector|MakeVector (.x _returnvalue_6) (.y _returnvalue_6) (Variables|Default|GetSpawnZ)) "0, 0, 0" false))
  ;[1 1 1] Set the reference to the spawner that generates the mob
  (bind _asenemy (Utilities|Casting|CastToEnemy _returnvalue_7))
  (Variables|/Game/Blueprints/AI/Enemy.Enemy_C|SetGeneratedBy _asenemy self))