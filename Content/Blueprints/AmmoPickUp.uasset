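; Ammo pickup actor that tops up the first-person character's ammo when touched.
; It spins continuously on all three axes in Tick.
; On overlap with a FirstPersonCharacter, it adds AmmoAmount clamped to that character's MaxAmmo, plays a collapse sound and explosion particle at its location, then destroys itself.
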(event EventBeginPlay)

(event Collision|EventActorBeginOverlap
  (params (OtherActor :type Actor%20Object%20Reference))
  (bind _returnvalue (Transformation|GetActorLocation))
  (bind _asfirst_person_character (Utilities|Casting|CastToFirstPersonCharacter OtherActor))
  (Variables|/Game/Blueprints/FirstPersonCharacter.FirstPersonCharacter_C|SetAmmo _asfirst_person_character (Math|Integer|Min(Integer) (+ (Variables|/Game/Blueprints/FirstPersonCharacter.FirstPersonCharacter_C|GetAmmo _asfirst_person_character) (Variables|Default|GetAmmoAmount)) (Variables|/Game/Blueprints/FirstPersonCharacter.FirstPersonCharacter_C|GetMaxAmmo _asfirst_person_character)))
  (Audio|PlaySoundatLocation "/Game/StarterContent/Audio/Collapse01.Collapse01" _returnvalue "0, 0, 0" 1.0 1.0 0.0 0 0 0)
  (Effects|SpawnEmitteratLocation "/Game/StarterContent/Particles/P_Explosion.P_Explosion" _returnvalue)
  (Actor|DestroyActor))

(event EventTick
  (params (DeltaSeconds :type Float%20%28single-precision%29))
  ;[1 1 1] Continuous rotate
  (Transformation|AddActorLocalRotation (* (Math|Rotator|MakeRotator 1.5e+02 72.0 1.5e+02) DeltaSeconds) false false))

(fn ConstructionScript)